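; Sound-control Blueprint for loop_amorph_1 that animates an audio component's crossfade and volume once play begins.
; The 0To1 timeline outputs curve values, feeding one to the sound's "crossFade" float parameter and the other to its volume multiplier.
; On-screen debug prints show both values, with the crossfade text colored green or red around the halfway point.
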(event EventBeginPlay
  ;[1 0.744 0] Parabel die den Float ausgibt
  (bind (_direction _crossfade_float _volume_multi_track) (Timeline|0%20to%201 Play)
    (:Update
      (Utilities|FlowControl|Sequence
        (:then_0
          ;[1 0.05561 0.6417] conPrint
          (bind _output_get (Variables|Default|SetFloat_Cross (* _crossfade_float 1.0)))
          (Utilities|FlowControl|Sequence
            (:then_0
              (Development|PrintString (Utilities|String|JoinStringArray (Utilities|Array|MakeArray (Variables|Default|GetCrossfade) (Utilities|String|ToString(Float) _output_get)) (Variables|Default|Getseperator)) (<= _output_get 0.5) false "(R=0.074610,G=0.471049,B=0.050510,A=1.000000)" (stale _output_get_2))
              (Audio|Parameter|SetFloatParameter (Variables|Components|GetAudioComponent) "crossFade" _output_get :!class /Script/Engine.AudioComponent :!label _label))
            (:then_1
              (Development|PrintString (Utilities|String|JoinStringArray (Utilities|Array|MakeArray (Variables|Default|GetCrossfade) (Utilities|String|ToString(Float) _output_get)) (Variables|Default|Getseperator)) (>= _output_get 0.5) false "(R=0.755208,G=0.031054,B=0.005930,A=1.000000)" (stale _output_get_2))
              (goto _label))
            (:then_2
              (bind _output_get_2 (Variables|Default|SetDur (Variables|Default|GetDur))))))
        (:then_1
          (Development|PrintString (Utilities|String|JoinStringArray (Utilities|Array|MakeArray (Variables|Default|Getvolume) (Utilities|String|ToString(Float) _volume_multi_track)) (Variables|Default|Getseperator)) true false "(R=0.755208,G=0.031054,B=0.005930,A=1.000000)")
          (Audio|Components|Audio|SetVolumeMultiplier (Variables|Components|GetAudioComponent) _volume_multi_track :!class /Script/Engine.AudioComponent))))))

(fn ConstructionScript)